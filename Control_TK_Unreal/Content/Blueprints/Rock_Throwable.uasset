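; Throwable rock actor that prepares its static mesh to be thrown.
; On BeginPlay it becomes movable, takes a custom collision object type and sets physics simulation from the SetPhysics variable.
; Each Tick sets CanThrow through a substring check that compares the mesh's collision type name with itself, so it normally always passes.
; A debug print of that check is left unconnected.
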(event EventBeginPlay
  (bind _staticmeshcomponent (Variables|Debug|GetStaticMeshComponent))
  ;[1 1 1] Setting an object up to be thrown
  (Collision|SetCollisionObjectType _staticmeshcomponent "ECC_GameTraceChannel4")
  (Transformation|SetMobility "Movable")
  (Physics|SetSimulatePhysics _staticmeshcomponent (Variables|Default|GetsetPhysics)))

(event EventTick
  (params (DeltaSeconds :type Float%20%28single-precision%29))
  (bind _staticmeshcomponent (Variables|Debug|GetStaticMeshComponent))
  (bind _returnvalue (Collision|GetCollisionObjectType _staticmeshcomponent))
  ;[1 1 1] Setting an object up to be thrown
  (bind _output_get (Variables|Default|SetCollisionObject (Utilities|String|EnumtoString _returnvalue)))
  (if (Utilities|String|Contains _output_get (Utilities|String|EnumtoString _returnvalue))
    (Variables|Default|SetcanThrow true)))

(fn ConstructionScript)